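; EnemyAI_BP is an enemy character that detects players with two colliders and passes the results to its EnemyController.
; The kill collider toggles IsPlayerDead, which per the author's note triggers a behavior-tree respawn at a random target point.
; The dash collider raises walk speed for players and uses a DoOnce to lock one overlapped actor as target.
; That actor leaving restores slow speed, clears the controller's target and resets the lock.
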(event `self.PlayerKillCollider.OnComponentBeginOverlap`
  (params (OverlappedComponent :type "PrimitiveComponent Object Reference") (OtherActor :type "Actor Object Reference") (OtherComp :type "PrimitiveComponent Object Reference") (OtherBodyIndex :type Integer) (bFromSweep :type Boolean) (SweepResult :type "HitResult Structure (by ref)"))
  ;[1 1 1] cheks if player is hit, if hit spawns AI to random targetpoint in behavior tree
  (if (`self.ActorHasTag` OtherActor "player")
    (bind _asenemy_controller (cast `/Game/AI/EnemyController` (`self.GetController`)))
    (set `/Game/AI/EnemyController.IsPlayerDead` true _asenemy_controller)))

(event `self.PlayerKillCollider.OnComponentEndOverlap`
  (params (OverlappedComponent :type "PrimitiveComponent Object Reference") (OtherActor :type "Actor Object Reference") (OtherComp :type "PrimitiveComponent Object Reference") (OtherBodyIndex :type Integer))
  ;[1 1 1] cheks if player is hit, if hit spawns AI to random targetpoint in behavior tree
  (bind _asenemy_controller (cast `/Game/AI/EnemyController` (`self.GetController`)))
  (set `/Game/AI/EnemyController.IsPlayerDead` false _asenemy_controller))

(event `self.DashCollider.OnComponentEndOverlap`
  (params (OverlappedComponent :type "PrimitiveComponent Object Reference") (OtherActor :type "Actor Object Reference") (OtherComp :type "PrimitiveComponent Object Reference") (OtherBodyIndex :type Integer))
  (bind _returnvalue (`self.GetController`))
  (bind _returnvalue_2 (`self.GetController`))
  ;[1 1 1] colliders for dash
  (if (`KismetTextLibrary.EqualEqual_TextText` (`KismetTextLibrary.Conv_StringToText` (`KismetSystemLibrary.GetObjectName` OtherActor)) (`KismetTextLibrary.Conv_StringToText` (`KismetSystemLibrary.GetObjectName` (`self.overlappedActor`))))
    (set `CharacterMovementComponent.MaxWalkSpeed` 100.0 (`self.CharacterMovement`))
    (bind _asenemy_controller (cast `/Game/AI/EnemyController` _returnvalue))
    (set `/Game/AI/EnemyController.BoolKey` false _asenemy_controller)
    (bind _asenemy_controller_2 (cast `/Game/AI/EnemyController` _returnvalue))
    (set `/Game/AI/EnemyController.OverlappedActors` (`self.overlappedActor_null`) _asenemy_controller_2)
    (goto _label :!via `Reset`)))

(event `self.DashCollider.OnComponentBeginOverlap`
  (params (OverlappedComponent :type "PrimitiveComponent Object Reference") (OtherActor :type "Actor Object Reference") (OtherComp :type "PrimitiveComponent Object Reference") (OtherBodyIndex :type Integer) (bFromSweep :type Boolean) (SweepResult :type "HitResult Structure (by ref)"))
  (bind _returnvalue (`self.GetController`))
  ;[1 1 1] colliders for dash
  (if (`self.ActorHasTag` OtherActor "player")
    (set `CharacterMovementComponent.MaxWalkSpeed` 500.0 (`self.CharacterMovement`))
    (`/Engine/EditorBlueprintResources/StandardMacros.DoOnce` false :!label _label
      (:`Completed`
        (bind _output_get (set `self.overlappedActor` OtherActor))
        (bind _asenemy_controller (cast `/Game/AI/EnemyController` _returnvalue))
        (set `/Game/AI/EnemyController.BoolKey` true _asenemy_controller)
        (bind _asenemy_controller_2 (cast `/Game/AI/EnemyController` _returnvalue)
          (:`then`
            (set `/Game/AI/EnemyController.OverlappedActors` _output_get _asenemy_controller_2))
          (:`CastFailed`
            (`KismetSystemLibrary.PrintText` "failed")))))))

(fn `UserConstructionScript`)