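; GreenArenaMode sets up a local multiplayer arena in which player characters are cabled to a shared tether core.
; On BeginPlay it gathers PlayerStarts, creates local players up to MaxPlayerCount, then spawns and possesses a character for each PlayerControllerBP.
; Each controller receives its index and start point, matched by array order.
; Finally it spawns TetherCoreBP at TetherSpawnPos and attaches cables to the spawned characters.
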(event `self.ReceiveBeginPlay`
  (`self.GetPlayerStartPoints`)
  (`self.SpawnPlayers`)
  (bind _returnvalue (`|SpawnActorFromClass` :`Class` "/Game/Blueprints/TetherCoreBP.TetherCoreBP_C" :`SpawnTransform` (`self.TetherSpawnPos`) :`CollisionHandlingOverride` "AlwaysSpawn" :`TransformScaleMethod` "OverrideRootScale" :`Instigator` null))
  (`/Game/Blueprints/TetherCoreBP.AttachCables` _returnvalue (`self.PlayersArray`)))

(fn `GetPlayerStartPoints`
  (bind _outactors (`GameplayStatics.GetAllActorsOfClass` "/Script/Engine.PlayerStart"))
  (set `self.PlayerStartArray` _outactors))

(fn `SpawnPlayers`
  (for _index (range 1 (`self.MaxPlayerCount`))
    (bind _returnvalue (`GameplayStatics.CreatePlayer` _index))
    (`KismetSystemLibrary.PrintString` (`KismetSystemLibrary.GetDisplayName` _returnvalue)))
  (bind _outactors (`GameplayStatics.GetAllActorsOfClass` "/Game/Blueprints/PlayerControllerBP.PlayerControllerBP_C"))
  (for (_array_element _array_index) _outactors
    (bind _asplayer_controller_bp (cast `/Game/Blueprints/PlayerControllerBP` _array_element))
    (bind _output (`|GetArrayItem` (`self.PlayerStartArray`) _array_index))
    (bind _returnvalue_2 (`|SpawnActorFromClass` "/Game/Blueprints/PlayerCharBP.PlayerCharBP_C" (`self.GetTransform` _output) "AlwaysSpawn" "OverrideRootScale" null null))
    (`Controller.Possess` _asplayer_controller_bp _returnvalue_2)
    (`KismetArrayLibrary.Array_AddUnique` (`self.PlayersArray`) _returnvalue_2)
    (`/Game/Blueprints/PlayerControllerBP.SetPlayerIndex` _asplayer_controller_bp _array_index)
    (`/Game/Blueprints/PlayerControllerBP.SetStartPos` _asplayer_controller_bp _output)))

(fn `UserConstructionScript`)