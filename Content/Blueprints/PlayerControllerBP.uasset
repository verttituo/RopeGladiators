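; Player controller that handles yaw-relative movement, a dash with cooldown, and a tether pull on the controlled pawn.
; Dash input calls speed-up on PlayerCharBP, while Tick counts down per-frame timers to end the boost and cooldown, printing debug messages.
; TetherDrag stores a normalized direction and clamped strength, which Tick applies as movement input every frame.
; Other events show or hide and disable the pawn, set its player index, and reset it to a start position.
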(event `EnablePlayer`
  (bind _returnvalue (`self.K2_GetPawn`))
  (`SceneComponent.SetHiddenInGame` (`self.GetComponentByClass` _returnvalue "/Script/Engine.MeshComponent") false true)
  (`self.SetActorEnableCollision` _returnvalue true)
  (`self.SetActorTickEnabled` _returnvalue true)
  (set `self.PlayerIsHidden` false))

(event `DisablePlayer`
  (bind _returnvalue (`self.K2_GetPawn`))
  (`SceneComponent.SetHiddenInGame` (`self.GetComponentByClass` _returnvalue "/Script/Engine.MeshComponent") true true)
  (`self.SetActorEnableCollision` _returnvalue false)
  (`self.SetActorTickEnabled` _returnvalue false)
  (set `self.PlayerIsHidden` true))

(event `SetPlayerIndex`
  (params (PlayerIndex :type Integer))
  (set `self.PlayerIndex` PlayerIndex))

(event `SetStartPos`
  (params (PawnStartPos :type "PlayerStart Object Reference"))
  (set `self.PawnStartPos` PawnStartPos))

(event `ResetToStartPos`
  (`self.K2_SetActorLocation` (`self.K2_GetPawn`) (`SceneComponent.K2_GetComponentLocation` (`Actor.RootComponent` (`self.PawnStartPos`))) false false))

(event `self.ReceiveTick`
  (params (DeltaSeconds :type "Float (single-precision)"))
  (`|ExecutionSequence`
    (:`then_0`
      (if (`self.DashSpeedUpActive`)
        (bind _result (`/Engine/EditorBlueprintResources/StandardMacros.DecrementFloat` (`self.DashSpeedUpTimer`))
          (:`  `
            (if (not (> _result 0.0))
              (set `self.DashSpeedUpActive` false)
              (set `self.DashSpeedUpTimer` (`self.DashSpeedUpDuration`))
              (bind _asplayer_char_bp (cast `/Game/Blueprints/PlayerCharBP` (`self.K2_GetPawn`)))
              (`/Game/Blueprints/PlayerCharBP.DashSpeedDown` _asplayer_char_bp))))))
    (:`then_1`
      (if (`self.DashActivated`)
        (bind _result_2 (`/Engine/EditorBlueprintResources/StandardMacros.DecrementFloat` (`self.DashCdTimer`))
          (:`  `
            (if (not (> _result_2 0.0))
              (set `self.DashActivated` false)
              (`KismetSystemLibrary.PrintString` (`KismetStringLibrary.Concat_StrStr` (`KismetStringLibrary.Conv_ObjectToString` (`self.K2_GetPawn`)) "Dash cooldown Done!")))))))
    (:`then_2`
      (`Pawn.AddMovementInput` (`self.K2_GetPawn`) (`self.TetherDragDirection`) (`self.TetherDragValue`) false))))

(event `InputAction|Dash`
  (params (Key :type "Key Structure"))
  (bind _returnvalue (`KismetStringLibrary.Conv_ObjectToString` (`self.K2_GetPawn`)))
  (:`Pressed`
    (if (`self.DashActivated`)
      (`KismetSystemLibrary.PrintString` (`KismetStringLibrary.Concat_StrStr` _returnvalue "Dash on Cooldown!"))
      (else
        (`KismetSystemLibrary.PrintString` (`KismetStringLibrary.Concat_StrStr` _returnvalue " Dash activated!"))
        (set `self.DashActivated` true)
        (set `self.DashSpeedUpActive` true)
        (set `self.DashCdTimer` (`self.DashCd`))
        (set `self.DashSpeedUpTimer` (`self.DashSpeedUpDuration`))
        (bind _asplayer_char_bp (cast `/Game/Blueprints/PlayerCharBP` (`self.K2_GetPawn`)))
        (`/Game/Blueprints/PlayerCharBP.DashSpeedUp` _asplayer_char_bp)))))

(event `InputAxis|MoveForward`
  (params (AxisValue :type "Float (single-precision)"))
  (bind (_returnvalue_roll _returnvalue_pitch _returnvalue_yaw) (`KismetMathLibrary.BreakRotator` (`Pawn.GetControlRotation` (`self.K2_GetPawn`))))
  (`Pawn.AddMovementInput` (`self.K2_GetPawn`) (`KismetMathLibrary.GetForwardVector` (`KismetMathLibrary.MakeRotator` 0.0 0.0 _returnvalue_yaw)) AxisValue false))

(event `InputAxis|MoveRight`
  (params (AxisValue :type "Float (single-precision)"))
  (bind (_returnvalue_roll _returnvalue_pitch _returnvalue_yaw) (`KismetMathLibrary.BreakRotator` (`Pawn.GetControlRotation` (`self.K2_GetPawn`))))
  (`Pawn.AddMovementInput` (`self.K2_GetPawn`) (`KismetMathLibrary.GetRightVector` (`KismetMathLibrary.MakeRotator` 0.0 0.0 _returnvalue_yaw)) AxisValue false))

(event `TetherDrag`
  (params (AxisValue :type "Float (double-precision)" :default 0.0) (DragDirection :type "Vector Structure"))
  (set `self.TetherDragDirection` (`KismetMathLibrary.Normal` DragDirection))
  (set `self.TetherDragValue` (`KismetMathLibrary.FClamp` AxisValue 0.0)))

(fn `UserConstructionScript`)