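; PlayerCharBP is the player character Blueprint, providing a dash speed toggle for character movement.
; Two events, DashSpeedUp and DashSpeedDown, swap the CharacterMovement max walk speed and acceleration between dash and normal variables.
; The graph holds no input binding or timing for these events, and the construction script is empty.
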(event `DashSpeedUp`
  (set `CharacterMovementComponent.MaxWalkSpeed` (`self.DashSpeed`) (`self.CharacterMovement`))
  (set `CharacterMovementComponent.MaxAcceleration` (`self.DashAccel`) (`self.CharacterMovement`)))

(event `DashSpeedDown`
  (set `CharacterMovementComponent.MaxWalkSpeed` (`self.NormalSpeed`) (`self.CharacterMovement`))
  (set `CharacterMovementComponent.MaxAcceleration` (`self.NormalAccel`) (`self.CharacterMovement`)))

(fn `UserConstructionScript`)