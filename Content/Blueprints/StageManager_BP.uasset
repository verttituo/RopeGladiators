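; Stage manager Blueprint that triggers timed trap spawns while spawning is switched on.
; StartSpawnTraps and EndSpawnTraps open and close a gate on Tick, which divides game time by SpawnTimer into a whole count.
; When that count divides evenly by GameTimeDivisor, a DoOnce fires TrapSpawn, re-arming on non-matching counts.
; A TODO notes that the spawn timer still needs resetting at the result screen.
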(event `self.ReceiveTick`
  (params (DeltaSeconds :type "Float (single-precision)"))
  (`/Engine/EditorBlueprintResources/StandardMacros.Gate` true :!label _label
    (:`Exit`
      (bind _output_get (set `self.EnableTrigger` (`KismetMathLibrary.Conv_IntToDouble` (`.ReturnValue` (`KismetMathLibrary.FMod` (`KismetSystemLibrary.GetGameTimeInSeconds`) (`self.SpawnTimer`))))))
      (if (== (`KismetMathLibrary.FMod` _output_get (`self.GameTimeDivisor`)) 0.0)
        (`/Engine/EditorBlueprintResources/StandardMacros.DoOnce` false :!label _label_2
          (:`Completed`
            (`self.TrapSpawn`)))
        (else
          (goto _label_2 :!via `Reset`))))))

(event `StartSpawnTraps`
  (goto _label :!via `Open`))

(event `EndSpawnTraps`
  (goto _label :!via `Close`))

(fn `UserConstructionScript`)