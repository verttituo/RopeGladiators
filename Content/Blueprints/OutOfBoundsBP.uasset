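; Out-of-bounds volume that reports a player hit to the GreenArenaMode game mode when a player overlaps it.
; On overlap, it identifies players by a case-sensitive "Player" substring in the actor's name, then passes that actor to PlayerGotHit.
; Custom events toggle the OutOfBoundsBox component's active state, with activation following a half-second delay.
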(event `DeActivateCollider`
  (`ActorComponent.SetActive` (`self.OutOfBoundsBox`) false false))

(event `ActivateCollider`
  (`KismetSystemLibrary.Delay` 0.5)
  (`ActorComponent.SetActive` (`self.OutOfBoundsBox`) true false))

(event `self.ReceiveActorBeginOverlap`
  (params (OtherActor :type "Actor Object Reference"))
  (if (`KismetStringLibrary.Contains` (`KismetStringLibrary.Conv_ObjectToString` OtherActor) "Player" true)
    (bind _asgreen_arena_mode (cast `/Game/Blueprints/GreenArenaMode` (`GameplayStatics.GetGameMode`)))
    (`/Game/Blueprints/GreenArenaMode.PlayerGotHit` _asgreen_arena_mode OtherActor)))

(fn `UserConstructionScript`)