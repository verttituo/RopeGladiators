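; Shared arena camera that frames up to four players from GreenArenaMode and becomes the view target for the PlayerControllerBP controllers.
; A fast looping timer, started on BeginPlay, sets spring arm length to the largest pairwise player distance, clamped to limits.
; It also eases the actor toward the raised average player position with VInterpTo.
; Invalid players add zero, yet the average still divides by the full player array length.
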(event `self.ReceiveBeginPlay`
  (`self.ClassSetup`)
  (`KismetSystemLibrary.K2_SetTimer` null "UpdateCamera" 0.001 true))

(event `UpdateCamera`
  (`self.SetArmLenght`)
  (`self.SetCameraPos`))

(fn `CalculateDistance`
  (params (PlayerRef1 :type "/Game/Blueprints/PlayerCharBP Object Reference") (PlayerRef2 :type "/Game/Blueprints/PlayerCharBP Object Reference"))
  (returns (Distance1 :type "Float (double-precision)"))
  (locals (Distance :type "Float (double-precision)" :default 0.0))
  (if (and (`KismetSystemLibrary.IsValid` PlayerRef1) (`KismetSystemLibrary.IsValid` PlayerRef2))
    (set `local.Distance` (`self.GetDistanceTo` PlayerRef1 PlayerRef2))
    (else
      (set `local.Distance` 0.0)))
  (return (`local.Distance`)))

(fn `ClassSetup`
  (bind _asgreen_arena_mode (cast `/Game/Blueprints/GreenArenaMode` (`GameplayStatics.GetGameMode`)))
  (bind _output_get (set `self.ArenaGameMode` _asgreen_arena_mode))
  (set `self.PlayersArrayRef` (`/Game/Blueprints/GreenArenaMode.PlayersArray` _output_get))
  (bind _outactors (`GameplayStatics.GetAllActorsOfClass` "/Game/Blueprints/PlayerControllerBP.PlayerControllerBP_C"))
  (`PlayerController.SetViewTargetWithBlend` _outactors self 0.0 "VTBlend_Linear" 0.0 false)
  (for (_array_element _array_index) (`self.PlayersArrayRef`)
    (switch `int` _array_index
      (:`0`
        (set `self.Player1` _array_element))
      (:`1`
        (set `self.Player2` _array_element))
      (:`2`
        (set `self.Player3` _array_element))
      (:`3`
        (set `self.Player4` _array_element)))))

(fn `GetLocation`
  (params (Player :type "/Game/Blueprints/PlayerCharBP Object Reference"))
  (returns (PlayerLocation :type "Vector Structure"))
  (locals (Location :type "Vector Structure" :default (0.0 0.0 0.0)))
  (`/Engine/EditorBlueprintResources/StandardMacros.IsValid` Player
    (:`Is Valid`
      (set `local.Location` (`self.K2_GetActorLocation` Player)))
    (:`Is Not Valid`
      (set `local.Location` (0.0 0.0 0.0))))
  (return (`local.Location`)))

(fn `SetArmLenght`
  (bind _player1 (`self.Player1`))
  (bind _player2 (`self.Player2`))
  (bind _player3 (`self.Player3`))
  (bind _player4 (`self.Player4`))
  (set `SpringArmComponent.TargetArmLength` (`KismetMathLibrary.FClamp` (`.MaxValue` (`KismetMathLibrary.MaxOfFloatArray` (`|MakeArray` (`self.CalculateDistance` _player1 _player2) (`self.CalculateDistance` _player1 _player3) (`self.CalculateDistance` _player1 _player4) (`self.CalculateDistance` _player2 _player3) (`self.CalculateDistance` _player2 _player4) (`self.CalculateDistance` _player3 _player4)))) (`self.MinArmLength`) (`self.MaxArmLenght`)) (`self.CameraSpringArm`)))

(fn `SetCameraPos`
  (set `self.TargetPos` (+ (/ (+ (`self.GetLocation` (`self.Player1`)) (`self.GetLocation` (`self.Player2`)) (`self.GetLocation` (`self.Player3`)) (`self.GetLocation` (`self.Player4`))) (`KismetMathLibrary.Conv_IntToDouble` (`KismetArrayLibrary.Array_Length` (`self.PlayersArrayRef`)))) (0.0 0.0 150.0)))
  (`self.K2_SetActorLocation` (`KismetMathLibrary.VInterpTo` (`self.PreviousPos`) (`self.TargetPos`) (`GameplayStatics.GetWorldDeltaSeconds`) (`self.InterpSpeed`)))
  (set `self.PreviousPos` (`self.K2_GetActorLocation`)))

(fn `UserConstructionScript`)