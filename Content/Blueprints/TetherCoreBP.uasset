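; Tether core actor that links up to four player characters with cables and floats between them, with events to attach, hide or show each cable.
; Each tick it finds the XY bounding-box midpoint of non-hidden players and feeds each controller a distance-based TetherDrag toward the core.
; Its capsule is pulled toward that midpoint by an elastic force growing with squared distance, switching to velocity damping within a minimum radius.
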(event `HideAttachedCable`
  (params (PlayerIndex :type Integer :default 0))
  (`SceneComponent.SetHiddenInGame` (`|GetArrayItem` (`self.CableArray`) PlayerIndex) true false))

(event `UnhideAttachedCable`
  (params (PlayerIndex :type Integer :default 0))
  (`SceneComponent.SetHiddenInGame` (`|GetArrayItem` (`self.CableArray`) PlayerIndex) false false))

(event `self.ReceiveBeginPlay`
  (bind _cablearray (`self.CableArray`))
  (`KismetArrayLibrary.Array_Add` _cablearray (`self.Cable1`))
  (`KismetArrayLibrary.Array_Add` _cablearray (`self.Cable2`))
  (`KismetArrayLibrary.Array_Add` _cablearray (`self.Cable3`))
  (`KismetArrayLibrary.Array_Add` _cablearray (`self.Cable4`))
  (for _array_element _cablearray
    (`SceneComponent.SetHiddenInGame` _array_element true false)))

(event `AttachCables`
  (params (PlayerCharsArray :type "Array of /Game/Blueprints/PlayerCharBP Object Reference"))
  (for (_array_element _array_index) PlayerCharsArray
    (bind _output (`|GetArrayItem` (`self.CableArray`) _array_index))
    (`CableComponent.SetAttachEndTo` _output _array_element "None" "None")
    (`SceneComponent.SetHiddenInGame` _output false false))
  (bind _outactors (`GameplayStatics.GetAllActorsOfClass` "/Game/Blueprints/PlayerControllerBP.PlayerControllerBP_C"))
  (bind _output_get (set `self.PlayerControllerArray` _outactors))
  (for _array_element_2 _output_get
    (bind _asplayer_char_bp (cast `/Game/Blueprints/PlayerCharBP` (`Controller.K2_GetPawn` _array_element_2)))
    (`KismetArrayLibrary.Array_Add` (`self.PlayerCharsArray`) _asplayer_char_bp)))

(event `self.ReceiveTick`
  (params (DeltaSeconds :type "Float (single-precision)"))
  (bind _elasticmultiplier (`self.ElasticMultiplier`))
  (bind _tetherspeedmultiplier (`self.TetherSpeedMultiplier`))
  (bind _ycoords (`self.YCoords`))
  (bind _xcoords (`self.XCoords`))
  (bind _tetherdampingmultiplier (`self.TetherDampingMultiplier`))
  (bind _returnvalue (- (`SceneComponent.K2_GetComponentLocation` (`self.Capsule`)) (`self.CenterPoint`)))
  (bind _returnvalue_2 (`KismetMathLibrary.VSize` _returnvalue))
  (bind (_returnvalue_x _returnvalue_y) (`KismetMathLibrary.BreakVector` (* (`SceneComponent.GetComponentVelocity` (`self.Capsule`)) (* (/ _returnvalue_2 (`self.MinDistance`)) -1.0))))
  (`self.ResetValues`) ; Reset Coordinate values
  (for _array_element (`self.PlayerCharsArray`)
    (bind _asplayer_controller_bp (cast `/Game/Blueprints/PlayerControllerBP` (`self.GetController` _array_element)))
    (if (not (`/Game/Blueprints/PlayerControllerBP.PlayerIsHidden` _asplayer_controller_bp))
      (bind (_returnvalue_x_2 _returnvalue_y_2 _returnvalue_z) (`KismetMathLibrary.BreakVector` (`self.K2_GetActorLocation` _array_element)))
      (`KismetArrayLibrary.Array_Add` (`self.YCoords`) _returnvalue_y_2)
      (`KismetArrayLibrary.Array_Add` (`self.XCoords`) _returnvalue_x_2)
      (bind _returnvalue_3 (`KismetMathLibrary.MakeVector` _returnvalue_x_2 _returnvalue_y_2 _returnvalue_z))
      (bind _returnvalue_4 (- (`SceneComponent.K2_GetComponentLocation` (`self.Capsule`)) _returnvalue_3))
      (bind _returnvalue_5 (`KismetMathLibrary.VSize` _returnvalue_4))
      (if (> (`self.PlayerDragMinDistance`) _returnvalue_5)
        (bind _returnvalue_6 (`self.GetController` _array_element))
        (bind _asplayer_controller_bp_2 (cast `/Game/Blueprints/PlayerControllerBP` _returnvalue_6))
        (`/Game/Blueprints/PlayerControllerBP.TetherDrag` _asplayer_controller_bp_2 0.0 _returnvalue_3)
        (else
          (bind _asplayer_controller_bp_3 (cast `/Game/Blueprints/PlayerControllerBP` _returnvalue_6))
          (`/Game/Blueprints/PlayerControllerBP.TetherDrag` _asplayer_controller_bp_3 (/ _returnvalue_5 400.0) _returnvalue_4)))))
  (set `self.CenterPoint` (`KismetMathLibrary.MakeVector` (/ (+ (`.MaxValue` (`KismetMathLibrary.MaxOfFloatArray` _xcoords)) (`.MinValue` (`KismetMathLibrary.MinOfFloatArray` _xcoords))) 2.0) (/ (+ (`.MaxValue` (`KismetMathLibrary.MaxOfFloatArray` _ycoords)) (`.MinValue` (`KismetMathLibrary.MinOfFloatArray` _ycoords))) 2.0)))
  (if (> (`self.MinDistance`) _returnvalue_2)
    (`PrimitiveComponent.AddForce` (`self.Capsule`) (`KismetMathLibrary.MakeVector` (* _tetherdampingmultiplier _returnvalue_x) (* _tetherdampingmultiplier _returnvalue_y)) "None" true)
    (else
      (set `self.ElasticMultiplier` (* _returnvalue_2 -2.0))
      (bind _output_get (set `self.TetherTickMovement` _returnvalue))
      (`PrimitiveComponent.AddForce` (`self.Capsule`) (`KismetMathLibrary.MakeVector` (* (.x _output_get) _elasticmultiplier _tetherspeedmultiplier) (* (.y _output_get) _elasticmultiplier _tetherspeedmultiplier)) "None" false))))

(fn `ResetValues`
  (set `self.TetherTickMovement` (0.0 0.0 0.0))
  (set `self.CenterPoint` (0.0 0.0 0.0))
  (set `self.MaxY` 0.0)
  (set `self.MaxX` 0.0)
  (`KismetArrayLibrary.Array_Clear` (`self.YCoords`))
  (`KismetArrayLibrary.Array_Clear` (`self.XCoords`))
  (set `self.ElasticMultiplier` 1.0)
  (set `self.CenterDamping` 1.0))

(fn `UserConstructionScript`)