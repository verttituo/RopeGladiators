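; Wall-mounted flamethrower hazard that sweeps back and forth through 180 degrees of yaw and hits players it touches.
; BeginPlay records the starting yaw and spawns a FlameParticles_Blueprint actor attached to the static mesh.
; Tick rotates the actor by a fixed per-frame step, flipping the RotateSide boolean after a short pause at each limit.
; Capsule overlaps with actors whose name contains "Player" call PlayerGotHit on GreenArenaMode.
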(event `self.ReceiveBeginPlay`
  (bind _staticmesh (`self.StaticMesh`))
  (bind (_relativerotation_roll _relativerotation_pitch _relativerotation_yaw) (`KismetMathLibrary.BreakRotator` (`SceneComponent.RelativeRotation` (`self.StaticMeshComponent`))))
  ;[1 1 1] Rotates wall flamethrower back and forth between 0-180 degrees on z-axis. Boolean is making the turn arounds
  (bind _output_get (set `self.FlametWallRot_Z` _relativerotation_yaw))
  (set `self.FlameWallOriginalRot` _output_get)
  (bind _returnvalue (`|SpawnActorFromClass` "/Game/Blueprints/FlameParticles_Blueprint.FlameParticles_Blueprint_C" (`SceneComponent.K2_GetComponentToWorld` _staticmesh) "Undefined" "OverrideRootScale" self null))
  (`self.K2_AttachToComponent` _returnvalue _staticmesh "None" "SnapToTarget" "SnapToTarget" "SnapToTarget" true))

(event `self.ReceiveTick`
  (params (DeltaSeconds :type "Float (single-precision)"))
  ;[1 1 1] Rotates wall flamethrower back and forth between 0-180 degrees on z-axis. Boolean is making the turn arounds
  (if (`self.Rotate+Side`)
    (if (< (`self.FlametWallRot_Z`) (+ (`self.FlameWallOriginalRot`) 180.0))
      (bind _output_get (set `self.FlametWallRot_Z` (+ (`self.FlametWallRot_Z`) 0.5)))
      (`self.K2_SetActorRotation` (`KismetMathLibrary.MakeRotator` 0.0 0.0 _output_get))
      (if (>= (`self.FlametWallRot_Z`) (+ (`self.FlameWallOriginalRot`) 180.0))
        (`KismetSystemLibrary.Delay` 1.0)
        (set `self.Rotate+Side` false)))
    (elif (> (`self.FlametWallRot_Z`) (`self.FlameWallOriginalRot`))
      (bind _output_get_2 (set `self.FlametWallRot_Z` (- (`self.FlametWallRot_Z`) 0.5)))
      (`self.K2_SetActorRotation` (`KismetMathLibrary.MakeRotator` 0.0 0.0 _output_get_2))
      (if (<= (`self.FlametWallRot_Z`) (`self.FlameWallOriginalRot`))
        (`KismetSystemLibrary.Delay` 1.0)
        (set `self.Rotate+Side` true)))))

(event `self.Capsule.OnComponentBeginOverlap`
  (params (OverlappedComponent :type "PrimitiveComponent Object Reference") (OtherActor :type "Actor Object Reference") (OtherComp :type "PrimitiveComponent Object Reference") (OtherBodyIndex :type Integer) (bFromSweep :type Boolean) (SweepResult :type "HitResult Structure (by ref)"))
  (if (`KismetStringLibrary.Contains` (`KismetStringLibrary.Conv_ObjectToString` OtherActor) "Player" true)
    (bind _asgreen_arena_mode (cast `/Game/Blueprints/GreenArenaMode` (`GameplayStatics.GetGameMode`)))
    (`/Game/Blueprints/GreenArenaMode.PlayerGotHit` _asgreen_arena_mode OtherActor)))

(fn `UserConstructionScript`)