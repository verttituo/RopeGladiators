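; DRay is a death ray hazard actor that widens over time and hits players it touches in the Green Arena mode.
; After a short delay, Tick grows its X and Y actor scale from the mesh's starting scale at fixed per-frame increments, capped for collider limits, until it self-destructs.
; On overlap, actors with "Player" in their name are reported to GreenArenaMode through PlayerGotHit.
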(event `self.ReceiveBeginPlay`
  (bind (_relativescale3d_x _relativescale3d_y) (`KismetMathLibrary.BreakVector` (`SceneComponent.RelativeScale3D` (`self.StaticMeshComponent`))))
  ;[1 1 1] Setting DRayMesh values to get static mesh components x&y scalevalues
  (set `self.DRayMesh_X` _relativescale3d_x)
  (set `self.DRayMesh_Y` _relativescale3d_y)
  (`KismetSystemLibrary.Delay` 1.5)
  (set `self.AllowExpand` true)
  (`KismetSystemLibrary.Delay` 4.5)
  (`self.K2_DestroyActor`))

(event `self.ReceiveTick`
  (params (DeltaSeconds :type "Float (single-precision)"))
  ;[1 1 1] Growing DeathRay as long as its meshs x scale size is smaller than 3
  (if (`self.AllowExpand`)
    (if (< (`self.DRayMesh_X`) 3.8)
      (bind _output_get (set `self.DRayMesh_X` (+ (`self.DRayMesh_X`) 0.01)))
      (bind _output_get_2 (set `self.DRayMesh_Y` (+ (`self.DRayMesh_Y`) 0.01)))
      (`self.SetActorScale3D` (`KismetMathLibrary.MakeVector` _output_get _output_get_2 16.0)))))

(event `self.ReceiveActorBeginOverlap`
  (params (OtherActor :type "Actor Object Reference"))
  (if (`KismetStringLibrary.Contains` (`KismetStringLibrary.Conv_ObjectToString` OtherActor) "Player" true)
    (bind _asgreen_arena_mode (cast `/Game/Blueprints/GreenArenaMode` (`GameplayStatics.GetGameMode`)))
    (`/Game/Blueprints/GreenArenaMode.PlayerGotHit` _asgreen_arena_mode OtherActor)))

(fn `UserConstructionScript`)