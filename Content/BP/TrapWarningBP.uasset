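; TrapWarningBP is a trap warning indicator that pulses the red intensity of its Cylinder mesh.
; BeginPlay creates a dynamic instance of WarningMat on the cylinder.
; Each Tick steps RedValue up or down, reversing via the FlipColor flag at fixed bounds, and writes it to the BaseColor parameter.
; The step is fixed per frame, so the pulse speed depends on frame rate.
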(event `self.ReceiveBeginPlay`
  (bind _returnvalue (`PrimitiveComponent.CreateDynamicMaterialInstance` (`self.Cylinder`) 0 "/Game/Materials/WarningMat.WarningMat"))
  (set `self.DynamicMat` _returnvalue))

(event `self.ReceiveTick`
  (params (DeltaSeconds :type "Float (single-precision)"))
  (if (`self.FlipColor`)
    (bind _output_get (set `self.RedValue` (+ (`self.RedValue`) 0.02)))
    (`MaterialInstanceDynamic.SetVectorParameterValue` (`self.DynamicMat`) "BaseColor" (make `LinearColor` _output_get 0.02 0.02))
    (if (> (`self.RedValue`) 1.0)
      (set `self.FlipColor` false))
    (else
      (bind _output_get_2 (set `self.RedValue` (- (`self.RedValue`) 0.02)))
      (`MaterialInstanceDynamic.SetVectorParameterValue` (`self.DynamicMat`) "BaseColor" (make `LinearColor` _output_get_2 0.02 0.02))
      (if (< (`self.RedValue`) 0.2)
        (set `self.FlipColor` true)))))

(fn `UserConstructionScript`)